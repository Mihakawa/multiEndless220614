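; Door actor that the player swings by holding the DragDoor input and turning.
; On press, a debug-drawn line trace from the character's camera flags the door as targeted if it hits any Drag_Door_BP, not specifically this instance.
; While held and targeted, Tick adds the character's TurnRate times Sensitivity to the door's yaw, within closed and open world-yaw limits.
; BeginPlay enables input and negates Sensitivity for flipped doors.
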(event `self.ReceiveTick`
  (params (DeltaSeconds :type "Float (single-precision)"))
  (bind (_returnvalue_roll _returnvalue_pitch _returnvalue_yaw) (`KismetMathLibrary.BreakRotator` (`SceneComponent.K2_GetComponentRotation` (`self.Door`))))
  ;[1 1 1] All checks to open the door
  (if (`self.IsHoldingLMB?`)
    (if (`self.IsLookingAtDoor?`)
      (if true
        (bind _returnvalue (* (`/Game/Blueprints/MyCharacter.Turn_Rate` (stale `InputAction|DragDoor` _asmy_character)) (`self.Sensitivity`)))
        (bind _returnvalue_2 (+ _returnvalue _returnvalue_yaw))
        (if (>= _returnvalue_2 (`self.Closed Angle Degrees`))
          (if (<= _returnvalue_2 (`self.Open Angle Degrees`))
            (`SceneComponent.K2_AddLocalRotation` (`self.Door`) (`KismetMathLibrary.MakeRotator` 0.0 0.0 _returnvalue) false false)))))))

(event `self.ReceiveBeginPlay`
  ;[1 1 1] Enable use of LMB
  (`self.EnableInput` (`GameplayStatics.GetPlayerController` 0))
  ;[1 1 1] Check if door is flipped
  (if (`self.Flipped`)
    (set `self.Sensitivity` (* (`self.Sensitivity`) -1.0))))

(event `InputAction|DragDoor`
  (params (Key :type "Key Structure"))
  ;[1 1 1] Check If Player Is Looking On The Door?
  (:`Pressed`
    (set `self.IsHoldingLMB?` true)
    (bind _asmy_character (cast `/Game/Blueprints/MyCharacter` (`GameplayStatics.GetPlayerCharacter` 0)))
    (bind _camera_position_ref (`/Game/Blueprints/MyCharacter.Camera Position Ref` _asmy_character))
    (bind _returnvalue (`SceneComponent.K2_GetComponentLocation` _camera_position_ref))
    (bind (_outhit _returnvalue_2) (`KismetSystemLibrary.LineTraceSingleForObjects` :`Start` _returnvalue :`End` (+ _returnvalue (* (`SceneComponent.GetForwardVector` _camera_position_ref) 500.0)) :`ObjectTypes` (`|MakeArray` "ObjectTypeQuery2" :!type "EObjectTypeQuery Enum") :`DrawDebugType` "ForDuration" :`bIgnoreSelf` false :`DrawTime` 1.0))
    (if _returnvalue_2
      (cast `/Game/Blueprints/Drag_Door_BP` (`.HitActor` (`GameplayStatics.BreakHitResult` _outhit)))
      (set `self.IsLookingAtDoor?` true)
      (else
        (set `self.IsLookingAtDoor?` false))))
  (:`Released`
    (set `self.IsHoldingLMB?` false)))

(fn `UserConstructionScript`)