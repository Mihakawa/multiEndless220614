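; Sliding window actor that raises or lowers a mesh with sound when the player presses Interact.
; A 500-unit camera line trace finds a mesh, whose relative Y selects opening or closing.
; Timelines lerp StatickMeshRef along Z, but its assignment from the hit mesh is disconnected.
; CanOpen blocks repeat input and resets only when closing finishes, so it stays false after opening.
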(event `self.ReceiveBeginPlay`
  (`self.EnableInput` (`GameplayStatics.GetPlayerController` 0)))

(event `InputAction|Interact`
  (params (Key :type "Key Structure"))
  (bind _returnvalue (`self.K2_GetActorLocation`))
  (bind (_relativelocation_x _relativelocation_y _relativelocation_z) (`KismetMathLibrary.BreakVector` (`SceneComponent.RelativeLocation` (`self.Statick mesh ref`))))
  (bind (_relativelocation_x_2 _relativelocation_y_2 _relativelocation_z_2) (`KismetMathLibrary.BreakVector` (`SceneComponent.RelativeLocation` (`self.Statick mesh ref`))))
  (:`Pressed`
    (if (`self.CanOpen?`)
      (set `self.CanOpen?` false)
      (bind _asmy_character (cast `/Game/Blueprints/MyCharacter` (`GameplayStatics.GetPlayerCharacter` 0)))
      (bind _camerafp (`/Game/Blueprints/MyCharacter.CameraFP` _asmy_character))
      (bind _returnvalue_2 (`SceneComponent.K2_GetComponentLocation` _camerafp))
      (bind (_outhit _returnvalue_3) (`KismetSystemLibrary.LineTraceSingleForObjects` :`Start` _returnvalue_2 :`End` (+ _returnvalue_2 (* (`SceneComponent.GetForwardVector` _camerafp) 500.0)) :`ObjectTypes` (`|MakeArray` "ObjectTypeQuery2" :!type "EObjectTypeQuery Enum") :`bIgnoreSelf` false))
      (if _returnvalue_3
        (bind _asstatic_mesh_component (cast `StaticMeshComponent` (`.HitComponent` (`GameplayStatics.BreakHitResult` _outhit))))
        (bind (_relativelocation_x_3 _relativelocation_y_3) (`KismetMathLibrary.BreakVector` (`SceneComponent.RelativeLocation` _asstatic_mesh_component)))
        (if (not (>= _relativelocation_y_3 50.0))
          (`GameplayStatics.PlaySoundAtLocation` "/Engine/VREditor/Sounds/UI/Dockable_Window_Open.Dockable_Window_Open" _returnvalue (struct) 1.0 1.0 0.0 null null null)
          (set `self.Start location` (`KismetMathLibrary.MakeVector` _relativelocation_x_2 _relativelocation_y_2 _relativelocation_z_2))
          (set `self.End location` (`KismetMathLibrary.MakeVector` _relativelocation_x_2 _relativelocation_y_2 (+ _relativelocation_z_2 50.0)))
          (bind (_direction _openwindow) (`Timeline|Timeline_0`)
            (:`Update`
              (`SceneComponent.K2_SetRelativeLocation` (`self.Statick mesh ref`) (`KismetMathLibrary.VLerp` (`self.Start location`) (`self.End location`) _openwindow) false false)))
          (else
            (`GameplayStatics.PlaySoundAtLocation` "/Engine/VREditor/Sounds/UI/Dockable_Window_Close.Dockable_Window_Close" _returnvalue (struct) 1.0 1.0 0.0 null null null)
            (set `self.Start location` (`KismetMathLibrary.MakeVector` _relativelocation_x _relativelocation_y _relativelocation_z))
            (set `self.End location` (`KismetMathLibrary.MakeVector` _relativelocation_x _relativelocation_y (+ _relativelocation_z -50.0)))
            (bind (_direction_2 _openwindow_2) (`Timeline|Timeline_1`)
              (:`Update`
                (`SceneComponent.K2_SetRelativeLocation` (`self.Statick mesh ref`) (`KismetMathLibrary.VLerp` (`self.Start location`) (`self.End location`) _openwindow_2) false false))
              (:`Finished`
                (set `self.CanOpen?` true)))))))))

(fn `UserConstructionScript`)